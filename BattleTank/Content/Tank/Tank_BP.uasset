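; Player-controllable tank Blueprint that wires input to movement and aiming components.
; BeginPlay hands the left and right tracks to TankMovement and the turret and barrel to TankAiming.
; Forward and Left axes send move and turn intents to TankMovement, and releasing Fire calls TankAiming.Fire.
; Aim axes rotate the camera rig, yawing AzimuthGimbal and pitching SpringArm, rather than moving the turret directly.
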(event EventBeginPlay
  (Class|TankMovementComponent|Initialize (Variables|Default|GetTankMovement) (Variables|Default|GetTrack%20Left) (Variables|Default|GetTrack%20Right))
  (Class|TankAimingComponent|Initialize (Variables|Default|GetTankAiming) (Variables|Default|GetTurret) (Variables|Default|GetTankBarrel)))

(event Input|ActionEvents|InputActionFire
  (params (Key :type Key%20Structure))
  (:Released
    (Class|TankAimingComponent|Fire (Variables|Default|GetTankAiming))))

(event Input|AxisEvents|InputAxisAimAzimuth
  (params (AxisValue :type Float%20%28single-precision%29))
  ;[1 1 1] Aim Input Binding
  (Transformation|AddLocalRotation (Variables|Default|GetAzimuthGimbal) (Math|Rotator|MakeRotator 0.0 0.0 AxisValue) false false))

(event Input|AxisEvents|InputAxisForward
  (params (AxisValue :type Float%20%28single-precision%29))
  ;[1 1 1] Controls to allow you to move with wasd
  (Class|TankMovementComponent|IntendMoveForward (Variables|Default|GetTankMovement) AxisValue))

(event Input|AxisEvents|InputAxisAimElevation
  (params (AxisValue :type Float%20%28single-precision%29))
  ;[1 1 1] Aim Input Binding
  (Transformation|AddLocalRotation (Variables|Default|GetSpringArm) (Math|Rotator|MakeRotator 0.0 AxisValue 0.0) false false))

(event Input|AxisEvents|InputAxisLeft
  (params (AxisValue :type Float%20%28single-precision%29))
  ;[1 1 1] Controls to allow you to move with wasd
  (Class|TankMovementComponent|IntendTurnLeft (Variables|Default|GetTankMovement) AxisValue))

(fn ConstructionScript)